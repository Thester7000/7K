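; Status effect component that applies freeze, paralysis, confusion, slowness, shrinking and a swiftness boost to its owning player.
; Interface events trigger timed effects using input disabling, time dilation, scale or walk speed changes, and UI overlays for some.
; Confusion and slowness swap Enhanced Input mapping contexts, with a slow-walk action applying scaled-down movement.
; Negative effects call a check on a shared flag and per-effect flags, reset after an immunity delay.
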(event `self.FreezePlayer`
  ;[1 1 1] Interface to activate effects
  (`self.Frozen`))

(event `Key|F`
  (params (Key :type "Key Structure")))

(event `self.ParalysePlayer`
  ;[1 1 1] Interface to activate effects
  (`self.Paralysis` 5))

(event `self.ConfusePlayer`
  ;[1 1 1] Interface to activate effects
  (`self.Confusion`))

(event `self.SlowPlayer`
  ;[1 1 1] Interface to activate effects
  (`self.Slowness`))

(event `self.ShrinkPlayer`
  ;[1 1 1] Interface to activate effects
  (`self.Shrinking`))

(event `self.ReceiveBeginPlay`
  ;[1 1 1] Setting Owner
  (set `self.OwnerRef` (`self.GetOwner`)))

(event `self.SwiftPlayer`
  ;[1 1 1] Interface to activate effects
  (`self.Swiftness`))

(event `Frozen`
  (bind _returnvalue (`GameplayStatics.GetPlayerController` 0))
  (bind _ui_fx_frozen (`self.UI_FX_FROZEN`))
  (bind _ownerref (`self.OwnerRef`))
  ;[1 1 1] Status Effect: Frozen
  (`self.StatusEffectCheck` (`self.CanBeFrozen`))
  (set `self.CanBeFrozen` false)
  (bind _returnvalue_2 (`|CreateWidget` "/StatusEffectPlugin/WBP_UI/WBP_UI_FX_FROZEN.WBP_UI_FX_FROZEN_C" (`GameplayStatics.GetPlayerController` 0)))
  (bind _output_get (set `self.UI_FX_FROZEN` _returnvalue_2))
  (`UserWidget.AddToViewport` _output_get 0)
  (`Widget.SetVisibility` _ui_fx_frozen "Visible")
  (`/StatusEffectPlugin/WBP_UI/WBP_UI_FX_FROZEN.FrozenAnimation` _ui_fx_frozen)
  (`Actor.DisableInput` _ownerref _returnvalue)
  (set `Actor.CustomTimeDilation` 0.0 _ownerref)
  (`KismetSystemLibrary.Delay` 1.6)
  (`Actor.EnableInput` _ownerref _returnvalue)
  (set `Actor.CustomTimeDilation` 1.0 _ownerref)
  (`Widget.SetVisibility` (`self.UI_FX_FROZEN`) "Hidden")
  (`KismetSystemLibrary.Delay` (`self.UnaffectedDuration`))
  (set `self.CanBeFrozen` true)
  (set `self.HasNegativeStatusEffect` false))

(event `Paralysis`
  (params (time :type Integer))
  (bind _returnvalue (`GameplayStatics.GetPlayerController` 0))
  (bind _ui_fx_paralysed (`self.UI_FX_PARALYSED`))
  (bind _ownerref (`self.OwnerRef`))
  ;[1 1 1] Status Effect: Paralysis
  (`self.StatusEffectCheck` (`self.CanBeParalysed`))
  (set `self.CanBeParalysed` false)
  (bind _returnvalue_2 (`|CreateWidget` "/StatusEffectPlugin/WBP_UI/WBP_UI_FX_PARALYSED.WBP_UI_FX_PARALYSED_C"))
  (set `self.UI_FX_PARALYSED` _returnvalue_2)
  (set `self.LoopNb` time)
  (if (< (`self.ParalysisIndex`) (`self.LoopNb`)) :!label _label
    (`UserWidget.AddToViewport` _ui_fx_paralysed 0)
    (`/StatusEffectPlugin/WBP_UI/WBP_UI_FX_PARALYSED.ParalysisAnimation` _ui_fx_paralysed)
    (`Actor.DisableInput` _ownerref _returnvalue)
    (`KismetSystemLibrary.Delay` 0.3)
    (`Actor.EnableInput` _ownerref _returnvalue)
    (`/Engine/EditorBlueprintResources/StandardMacros.IncrementInt` (`self.ParalysisIndex`)
      (:`  `
        (`Widget.RemoveFromParent` (`self.UI_FX_PARALYSED`))
        (`KismetSystemLibrary.Delay` 0.5)
        (goto _label)))
    (else
      (set `self.ParalysisIndex` 0)
      (`KismetSystemLibrary.Delay` (`self.UnaffectedDuration`))
      (set `self.CanBeParalysed` true)
      (set `self.HasNegativeStatusEffect` false))))

(event `Confusion`
  (bind _returnvalue (pcsubsystem `EnhancedInputLocalPlayerSubsystem` (`GameplayStatics.GetPlayerController` 0)))
  ;[1 1 1] Status Effect: Confusion
  (`self.StatusEffectCheck` (`self.CanBeConfused`))
  (set `self.CanBeConfused` false)
  (bind _returnvalue_2 (`|CreateWidget` "/StatusEffectPlugin/WBP_UI/WBP_UI_FX_CONFUSED.WBP_UI_FX_CONFUSED_C"))
  (bind _output_get (set `self.UI_FX_CONFUSED` _returnvalue_2))
  (`UserWidget.AddToViewport` _output_get 0)
  (`/StatusEffectPlugin/WBP_UI/WBP_UI_FX_CONFUSED.ConfusedAnimation` _output_get)
  (`EnhancedInputSubsystemInterface.RemoveMappingContext` _returnvalue "/StatusEffectPlugin/InputComponents/Base/IMC_GAD2010.IMC_GAD2010" (struct))
  (`EnhancedInputSubsystemInterface.AddMappingContext` _returnvalue "/StatusEffectPlugin/InputComponents/IMC_ConfusionWeak.IMC_ConfusionWeak" 0 (struct))
  (`KismetSystemLibrary.Delay` 3.0)
  (`EnhancedInputSubsystemInterface.RemoveMappingContext` _returnvalue "/StatusEffectPlugin/InputComponents/IMC_ConfusionWeak.IMC_ConfusionWeak" (struct))
  (`EnhancedInputSubsystemInterface.AddMappingContext` _returnvalue "/StatusEffectPlugin/InputComponents/Base/IMC_GAD2010.IMC_GAD2010" 0 (struct))
  (`Widget.RemoveFromParent` (`self.UI_FX_CONFUSED`))
  (`KismetSystemLibrary.Delay` (`self.UnaffectedDuration`))
  (set `self.CanBeConfused` true)
  (set `self.HasNegativeStatusEffect` false))

(event `Slowness`
  (bind _returnvalue (pcsubsystem `EnhancedInputLocalPlayerSubsystem` (`GameplayStatics.GetPlayerController` 0)))
  ;[1 1 1] Status Effect: Slowness
  (`self.StatusEffectCheck` (`self.CanBeSlowed`))
  (set `self.CanBeSlowed` false)
  (`EnhancedInputSubsystemInterface.RemoveMappingContext` _returnvalue "/StatusEffectPlugin/InputComponents/Base/IMC_GAD2010.IMC_GAD2010" (struct))
  (`EnhancedInputSubsystemInterface.AddMappingContext` _returnvalue "/StatusEffectPlugin/InputComponents/IMC_SlowWalk.IMC_SlowWalk" 0 (struct))
  (`KismetSystemLibrary.Delay` 3.5)
  (`EnhancedInputSubsystemInterface.RemoveMappingContext` _returnvalue "/StatusEffectPlugin/InputComponents/IMC_SlowWalk.IMC_SlowWalk" (struct))
  (`EnhancedInputSubsystemInterface.AddMappingContext` _returnvalue "/StatusEffectPlugin/InputComponents/Base/IMC_GAD2010.IMC_GAD2010" 0 (struct))
  (`KismetSystemLibrary.Delay` (`self.UnaffectedDuration`))
  (set `self.CanBeSlowed` true)
  (set `self.HasNegativeStatusEffect` false))

(event `EnhancedInput|/StatusEffectPlugin/InputComponents/IA_SlowWalk`
  (params (ActionValue :type "Vector2D Structure") (ElapsedSeconds :type "Float (double-precision)") (TriggeredSeconds :type "Float (double-precision)") (InputAction :type "InputAction Object Reference" :default "/StatusEffectPlugin/InputComponents/IA_SlowWalk.IA_SlowWalk"))
  ;[1 1 1] Status Effect: Slowness
  (:`Triggered`
    (`Pawn.AddMovementInput` (`Actor.Instigator` (`self.OwnerRef`)) (`self.InputForSpeedChange` ActionValue) 0.4 false)))

(event `Shrinking`
  (bind _ownerref (`self.OwnerRef`))
  ;[1 1 1] Status Effect: Shrinking
  (`self.StatusEffectCheck` (`self.CanBeShrunk`))
  (set `self.CanBeShrunk` false)
  (`Actor.SetActorScale3D` _ownerref (`KismetMathLibrary.Conv_DoubleToVector` (`self.New Scale 3D (SHRINK)`)))
  (`SceneComponent.K2_AddRelativeLocation` (`Actor.RootComponent` _ownerref) (0.0 0.0 -35.0) true false)
  (`KismetSystemLibrary.Delay` 4.0)
  (`SceneComponent.K2_AddRelativeLocation` (`Actor.RootComponent` _ownerref) (0.0 0.0 60.0) false false)
  (`Actor.SetActorScale3D` _ownerref (1.0 1.0 1.0))
  (`KismetSystemLibrary.Delay` (`self.UnaffectedDuration`))
  (set `self.CanBeShrunk` true)
  (set `self.HasNegativeStatusEffect` false))

(event `Swiftness`
  (bind _returnvalue (`Actor.GetComponentByClass` (`self.OwnerRef`) "/Script/Engine.CharacterMovementComponent"))
  ;[1 1 1] Status Effect: Swiftness
  (set `CharacterMovementComponent.MaxWalkSpeed` 900.0 _returnvalue)
  (`KismetSystemLibrary.Delay` 2.5)
  (set `CharacterMovementComponent.MaxWalkSpeed` 550.0 _returnvalue))

(fn `StatusEffectCheck`
  (params (StatusEffect :type Boolean))
  (if (== StatusEffect (not (`self.HasNegativeStatusEffect`)))
    (set `self.HasNegativeStatusEffect` true)))